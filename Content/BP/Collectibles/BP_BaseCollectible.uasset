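; BP_BaseCollectible is a base pickup that BP_HTKCharacter collects by overlapping its sphere.
; A Timeline, with Play called every Tick, drives the mesh's relative Z to animate it vertically.
; On overlap, GetCollected passes the item's Worth to CollectCoins on the HUD's collectibles widget for player 0, then disables sphere collision and destroys the actor.
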(event OnComponentBeginOverlap(Sphere)
  (params (OverlappedComponent :type Primitive%20Component%20Object%20Reference) (OtherActor :type Actor%20Object%20Reference) (OtherComp :type Primitive%20Component%20Object%20Reference) (OtherBodyIndex :type Integer) (bFromSweep :type Boolean) (SweepResult :type Hit%20Result%20Structure%20%28by%20ref%29))
  (Utilities|Casting|CastToBP_HTKCharacter OtherActor)
  (CallFunction|GetCollected))

(event Custom|Get%20Collected
  ;[0.15 0.15 0.15 0.5] Increase counter in UI
  (bind _asbp_hud (Utilities|Casting|CastToBP_HUD (HUD|GetHUD (Game|GetPlayerController 0))))
  (Default|CollectCoins (Variables|/Game/UI/BP_HUD.BP_HUD_C|GetCollectibles%20Widget _asbp_hud) (Variables|Default|GetWorth))
  (Collision|SetCollisionEnabled (Variables|Default|GetSphere) "NoCollision")
  (Actor|DestroyActor))

(event EventTick
  (params (DeltaSeconds :type Float%20%28single-precision%29))
  (bind _loc (Timeline|Timeline Play)
    (:Update
      (Transformation|SetRelativeLocation (Variables|Default|GetMesh) (Math|Vector|MakeVector 0.0 0.0 (* _loc 4e+01)) false false))))

(fn ConstructionScript)